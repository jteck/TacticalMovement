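; Thrown grenade projectile that bounces, then explodes when its fuse runs out, dealing radial damage with falloff.
; The construction script sets the mesh, material and bouncing projectile movement, and each bounce plays an impact sound.
; The server runs the fuse timer and applies damage, while a multicast event spawns the explosion effect and sound.
; After detonation it disables collision and hides itself, then destroys itself after a short delay.
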(event Custom|Detonate
  (Class|GameplayStatics|ApplyRadialDamagewithFalloff (Variables|Default|GetDamage) 0.0 (Transformation|GetActorLocation) 0.0 (Variables|Default|GetExplosion%20Radius) 1.0 (Variables|Default|GetDamage%20Type) 0 self (Game|GetInstigatorController) "ECC_Visibility")
  (CallFunction|MulticastDetonated)
  (Collision|SetCollisionEnabled (Variables|Default|GetCollisionComponent) "NoCollision")
  (Rendering|SetActorHiddenInGame true)
  (Utilities|FlowControl|Delay 0.15)
  (Actor|DestroyActor))

(event Custom|Multicast_Detonated
  (bind _returnvalue (Transformation|GetActorLocation))
  (Niagara|SpawnSystematLocation "/Game/Effects/Particles/Explosion/NS_Grenade_Explosion.NS_Grenade_Explosion" _returnvalue)
  (Audio|SpawnSoundatLocation "/Game/Audio/MetaSounds/sfx_Weapon_GrenadeExplosion_nl_meta.sfx_Weapon_GrenadeExplosion_nl_meta" _returnvalue "0, 0, 0" 1.0 1.0 0.0 "/Game/Audio/AttenuationPresets/ATT_Grenade.ATT_Grenade" 0))

(event Custom|OnProjectileBounce_Event
  (params (ImpactResult :type Hit%20Result%20Structure%20%28by%20ref%29) (ImpactVelocity :type Vector%20%28by%20ref%29))
  (Audio|SpawnSoundatLocation "/Game/Audio/MetaSounds/sfx_Weapon_GrenadeImpact_nl_meta.sfx_Weapon_GrenadeImpact_nl_meta" (Transformation|GetActorLocation) "0, 0, 0" 1.0 1.0 0.0 "/Game/Audio/AttenuationPresets/ATT_FX_GrenadeBounce.ATT_FX_GrenadeBounce" 0))

(event EventBeginPlay
  (|CallParentFunction)
  (EventDispatchers|AssignOnProjectileBounce (Variables|Default|GetProjectileMovement) (delegate Custom|OnProjectileBounce_Event))
  (if (Ability|HasAuthority)
    (Utilities|Time|SetTimerbyEvent (delegate Custom|Detonate) (Variables|Default|GetFuseTime))))

(fn ConstructionScript
  (bind _sphere (Variables|Default|GetSphere))
  (bind _projectilemovement (Variables|Default|GetProjectileMovement))
  (Components|StaticMesh|SetStaticMesh _sphere "/Game/Weapons/Grenade/Mesh/SM_grenade.SM_grenade")
  (Rendering|Material|SetMaterial _sphere 0 "/Game/Weapons/Grenade/Material/MI_Weapon_Grenade.MI_Weapon_Grenade")
  (Variables|/Script/Engine.ProjectileMovementComponent|SetInitialSpeed _projectilemovement 2.5e+03)
  (Variables|/Script/Engine.ProjectileMovementComponent|SetMaxSpeed _projectilemovement 2.55e+03)
  (Variables|/Script/Engine.ProjectileMovementComponent|SetProjectileGravityScale _projectilemovement 1.0)
  (Variables|/Script/Engine.ProjectileMovementComponent|SetbShouldBounce _projectilemovement true)
  (Variables|/Script/Engine.ProjectileMovementComponent|SetBounciness _projectilemovement 0.3)
  (Variables|/Script/Engine.ProjectileMovementComponent|SetFriction _projectilemovement 0.8)
  (Variables|/Script/Engine.ProjectileMovementComponent|SetBounceVelocityStopSimulatingThreshold _projectilemovement 25.0))